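; BP_Barrel is an interactable barrel that rotates between upright and tipped when moved, playing a sound each time.
; Its trigger registers it as NearBarrel on an overlapping BP_FirstPersonCharacter and shows the WBMove prompt, clearing both on exit.
; MoveBarrel toggles a state flag and plays or reverses a timeline that lerps the mesh rotation by up to 90 degrees.
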(event `MoveBarrel`
  (bind _returnvalue (`self.K2_GetActorLocation`))
  (if (`self.BarrelMoved`)
    (`GameplayStatics.PlaySoundAtLocation` null _returnvalue (struct) 1.0 1.0 0.0 null null null null)
    (set `self.BarrelMoved` false)
    (bind (_direction _alpha) (`Timeline|Barrel_Timeline` :!via `Reverse` :!label _label)
      (:`Update`
        (`SceneComponent.K2_SetRelativeLocationAndRotation` (`self.Barrel`) (0.0 0.0 0.0) (`KismetMathLibrary.RLerp` (struct) (struct :`Roll` 90.0) _alpha) false false)))
    (else
      (`GameplayStatics.PlaySoundAtLocation` null _returnvalue (struct) 1.0 1.0 0.0 null null null null)
      (set `self.BarrelMoved` true)
      (goto _label))))

(event `self.Trigger.OnComponentBeginOverlap`
  (params (OverlappedComponent :type "PrimitiveComponent Object Reference") (OtherActor :type "Actor Object Reference") (OtherComp :type "PrimitiveComponent Object Reference") (OtherBodyIndex :type Integer) (bFromSweep :type Boolean) (SweepResult :type "HitResult Structure (by ref)"))
  (bind _asbp_first_person_character (cast `/Game/FirstPerson/Blueprints/BP_FirstPersonCharacter` OtherActor))
  (set `/Game/FirstPerson/Blueprints/BP_FirstPersonCharacter.Near_Barrel` self _asbp_first_person_character)
  (`SceneComponent.SetVisibility` (`self.WB_Move`) true false))

(event `self.Trigger.OnComponentEndOverlap`
  (params (OverlappedComponent :type "PrimitiveComponent Object Reference") (OtherActor :type "Actor Object Reference") (OtherComp :type "PrimitiveComponent Object Reference") (OtherBodyIndex :type Integer))
  (bind _asbp_first_person_character (cast `/Game/FirstPerson/Blueprints/BP_FirstPersonCharacter` OtherActor))
  (set `/Game/FirstPerson/Blueprints/BP_FirstPersonCharacter.Near_Barrel` null _asbp_first_person_character)
  (`SceneComponent.SetVisibility` (`self.WB_Move`) false false))

(event `self.ReceiveBeginPlay`
  (`self.EnableInput` (`GameplayStatics.GetPlayerController` 0)))

(fn `UserConstructionScript`)