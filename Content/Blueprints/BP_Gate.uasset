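; BP_Gate is a hinged gate that the first-person player can open only while holding a key.
; Its trigger registers it as the character's NearGate and clears that on exit, also hiding the lock widget.
; Togglegate checks HasKey to open or show the lock widget, switches blocker collision, and swings the hinge by timeline.
; Open_Animation and Close_Animation share a separate keyless toggle that changes trigger collision instead.
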(event `Toggle gate`
  (if (`self.IsOpen`)
    (`PrimitiveComponent.SetCollisionEnabled` (`self.Gate Blocker`) "QueryAndPhysics")
    (set `self.IsOpen` false)
    (`GameplayStatics.PlaySoundAtLocation` null (`self.K2_GetActorLocation`) (struct) 1.0 1.0 0.0 null null null null)
    (bind (_direction _alpha) (`Timeline|Gate_Timeline` :!via `Reverse` :!label _label)
      (:`Update`
        (`SceneComponent.K2_SetRelativeLocationAndRotation` (`self.Hinge root`) (0.0 0.0 0.0) (`KismetMathLibrary.RLerp` (struct) (struct :`Yaw` 90.0) _alpha) false false)))
    (else
      (bind _asbp_first_person_character (cast `/Game/FirstPerson/Blueprints/BP_FirstPersonCharacter` (`GameplayStatics.GetPlayerCharacter` 0)))
      (if (`/Game/FirstPerson/Blueprints/BP_FirstPersonCharacter.HasKey` _asbp_first_person_character)
        (`GameplayStatics.PlaySoundAtLocation` null (0.0 0.0 0.0) (struct) 1.0 1.0 0.0 null null null null)
        (`PrimitiveComponent.SetCollisionEnabled` (`self.Gate Blocker`) "NoCollision")
        (set `self.IsOpen` true)
        (`GameplayStatics.PlaySoundAtLocation` null (`self.K2_GetActorLocation`) (struct) 1.0 1.0 0.0 null null null null)
        (goto _label)
        (else
          (`GameplayStatics.PlaySoundAtLocation` null (0.0 0.0 0.0) (struct) 1.0 1.0 0.0 null null null null)
          (`SceneComponent.SetVisibility` (`self.WB_GateLock`) true false))))))

(event `self.TriggerCollision.OnComponentBeginOverlap`
  (params (OverlappedComponent :type "PrimitiveComponent Object Reference") (OtherActor :type "Actor Object Reference") (OtherComp :type "PrimitiveComponent Object Reference") (OtherBodyIndex :type Integer) (bFromSweep :type Boolean) (SweepResult :type "HitResult Structure (by ref)"))
  (bind _asbp_first_person_character (cast `/Game/FirstPerson/Blueprints/BP_FirstPersonCharacter` OtherActor))
  (set `/Game/FirstPerson/Blueprints/BP_FirstPersonCharacter.NearGate` self _asbp_first_person_character))

(event `Open_Animation`
  (bind _triggercollision (`self.TriggerCollision`))
  (if (`self.IsOpen`) :!label _label_2
    (set `self.IsOpen` false)
    (`PrimitiveComponent.SetCollisionEnabled` _triggercollision "QueryAndPhysics")
    (`GameplayStatics.PlaySoundAtLocation` null (0.0 0.0 0.0) (struct) 1.0 1.0 0.0 null null null null)
    (bind (_direction _open) (`Timeline|Animation` :!via `Reverse` :!label _label_3)
      (:`Update`
        (`SceneComponent.K2_SetRelativeLocationAndRotation` (`self.Hinge root`) (0.0 0.0 0.0) (`KismetMathLibrary.RLerp` (struct) (struct :`Yaw` 90.0) _open) false false)))
    (else
      (set `self.IsOpen` true)
      (`PrimitiveComponent.SetCollisionEnabled` _triggercollision "NoCollision")
      (`GameplayStatics.PlaySoundAtLocation` null (0.0 0.0 0.0) (struct) 1.0 1.0 0.0 null null null null)
      (goto _label_3))))

(event `Close_Animation`
  (goto _label_2))

(event `self.TriggerCollision.OnComponentEndOverlap`
  (params (OverlappedComponent :type "PrimitiveComponent Object Reference") (OtherActor :type "Actor Object Reference") (OtherComp :type "PrimitiveComponent Object Reference") (OtherBodyIndex :type Integer))
  (bind _asbp_first_person_character (cast `/Game/FirstPerson/Blueprints/BP_FirstPersonCharacter` OtherActor))
  (set `/Game/FirstPerson/Blueprints/BP_FirstPersonCharacter.NearGate` null _asbp_first_person_character)
  (`SceneComponent.SetVisibility` (`self.WB_GateLock`) false false))

(event `self.ReceiveBeginPlay`
  (`self.EnableInput` (`GameplayStatics.GetPlayerController` 0)))

(fn `NewFunction`)

(fn `UserConstructionScript`)