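; BP_Key is a key pickup actor for the first-person character.
; Entering its Trigger registers the key as the character's NearKey, sets HasKey immediately and shows PickUpPrompt; leaving clears NearKey and hides the prompt.
; PickKey plays a shutter sound at the world origin and destroys the actor, or prints a notice if GotKey is set, which this graph never does.
; A touch event enables player input.
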(event `self.Trigger.OnComponentBeginOverlap`
  (params (OverlappedComponent :type "PrimitiveComponent Object Reference") (OtherActor :type "Actor Object Reference") (OtherComp :type "PrimitiveComponent Object Reference") (OtherBodyIndex :type Integer) (bFromSweep :type Boolean) (SweepResult :type "HitResult Structure (by ref)"))
  (bind _asbp_first_person_character (cast `/Game/FirstPerson/Blueprints/BP_FirstPersonCharacter` OtherActor))
  (set `/Game/FirstPerson/Blueprints/BP_FirstPersonCharacter.NearKey` self _asbp_first_person_character)
  (bind _output_get (set `/Game/FirstPerson/Blueprints/BP_FirstPersonCharacter.HasKey` true _asbp_first_person_character))
  (if _output_get
    (`SceneComponent.SetVisibility` (`self.PickUpPrompt`) true false)))

(event `PickKey`
  (if (`self.GotKey`)
    (`KismetSystemLibrary.PrintString` "Already Acquired Key")
    (else
      (`GameplayStatics.PlaySoundAtLocation` "/Engine/VREditor/Sounds/UI/Camera_Shutter.Camera_Shutter" (0.0 0.0 0.0) (struct) 1.0 1.0 0.0 null null null null)
      (`self.K2_DestroyActor`))))

(event `self.Trigger.OnComponentEndOverlap`
  (params (OverlappedComponent :type "PrimitiveComponent Object Reference") (OtherActor :type "Actor Object Reference") (OtherComp :type "PrimitiveComponent Object Reference") (OtherBodyIndex :type Integer))
  (bind _asbp_first_person_character (cast `/Game/FirstPerson/Blueprints/BP_FirstPersonCharacter` OtherActor))
  (set `/Game/FirstPerson/Blueprints/BP_FirstPersonCharacter.NearKey` null _asbp_first_person_character)
  (`SceneComponent.SetVisibility` (`self.PickUpPrompt`) false false))

(event `self.ReceiveActorOnInputTouchBegin`
  (params (FingerIndex :type "ETouchIndex Enum" :default "Touch1"))
  (`self.EnableInput` (`GameplayStatics.GetPlayerController` 0)))

(fn `UserConstructionScript`)