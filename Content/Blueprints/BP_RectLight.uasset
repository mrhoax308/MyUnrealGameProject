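; BP_RectLight is a room light Blueprint that can flicker when its Flicker_Start event is called and go dark on Flicker_Stop.
; Both events set a FlickeringStatus flag and use it as the light's visibility, so stopping hides the light entirely.
; While the flag is set, a self-calling FlickerLoop event randomizes intensity, waits a short random Delay, and repeats without using Tick.
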(event `Flicker_Stop`
  (bind _output_get (set `self.Flickering_Status` false))
  (`SceneComponent.SetVisibility` (`self.RoomLight`) _output_get false))

(event `Flicker_Start`
  (bind _output_get (set `self.Flickering_Status` true))
  (`SceneComponent.SetVisibility` (`self.RoomLight`) _output_get false)
  (`self.FlickerLoop`))

(event `FlickerLoop`
  (if (`self.Flickering_Status`)
    (`LightComponent.SetIntensity` (`self.RoomLight`) (`KismetMathLibrary.RandomFloatInRange` 50.0 4000.0))
    (`KismetSystemLibrary.Delay` (`KismetMathLibrary.RandomFloatInRange` 0.1 0.3))
    (`self.FlickerLoop`)))

(fn `UserConstructionScript`)